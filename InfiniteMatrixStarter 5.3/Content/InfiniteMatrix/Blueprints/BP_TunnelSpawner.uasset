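; Tunnel spawner actor that builds a chain of BP_Tunnel segments populated with enemies and pickups.
; On BeginPlay it clears existing tunnels and spawns a few, starting at the player pawn.
; SpawnTunnelAtPoint chains each segment to the newest one's SpawnPoint, and each segment receives a spawner reference and randomized wall.
; Each segment spawns a randomly offset enemy and sometimes a health pack; lifespans are set only when a pack spawns.
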(event `self.ReceiveBeginPlay`
  (`self.SpawnInitialTunnels`))

(fn `SpawnInitialTunnels`
  (`|ExecutionSequence`
    (:`then_0`
      (bind _outactors (`GameplayStatics.GetAllActorsOfClass` "/Game/InfiniteMatrix/Blueprints/BP_Tunnel.BP_Tunnel_C"))
      (for _array_element _outactors
        (`self.K2_DestroyActor` _array_element)))
    (:`then_1`
      (for _ (range 3)
        (`/Engine/EditorBlueprintResources/StandardMacros.IsValid` (`self.NewestTunnel`)
          (:`Is Valid`
            (`self.SpawnTunnelAtPoint`))
          (:`Is Not Valid`
            (`self.SpawnTunnel` (`self.K2_GetActorLocation` (`GameplayStatics.GetPlayerPawn` 0)))))))))

(fn `SpawnTunnel`
  (params (SpawnLocation :type "Vector Structure"))
  (bind _returnvalue (+ SpawnLocation (`KismetMathLibrary.MakeVector` (`KismetMathLibrary.RandomFloatInRange` 500.0 2000.0) (`KismetMathLibrary.RandomFloatInRange` -125.0 125.0) (`KismetMathLibrary.RandomFloatInRange` -125.0 125.0))))
  (bind _returnvalue_2 (`|SpawnActorFromClass` "/Game/InfiniteMatrix/Blueprints/BP_Tunnel.BP_Tunnel_C" (`KismetMathLibrary.MakeTransform` SpawnLocation) "Undefined" "MultiplyWithRoot" null null))
  (bind _output_get (set `self.NewestTunnel` _returnvalue_2))
  (set `/Game/InfiniteMatrix/Blueprints/BP_Tunnel.IsPassed` true _output_get)
  (set `/Game/InfiniteMatrix/Blueprints/BP_Tunnel.TunnelSpawner` self _output_get)
  (`/Game/InfiniteMatrix/Blueprints/BP_Tunnel.RandomizeWall` _output_get)
  (bind _returnvalue_3 (`|SpawnActorFromClass` "/Game/InfiniteMatrix/Blueprints/BP_Enemy.BP_Enemy_C" (`KismetMathLibrary.MakeTransform` _returnvalue) "Undefined" "MultiplyWithRoot" null null))
  (if (< (`KismetMathLibrary.RandomIntegerInRange` 0 10) 5)
    (bind _returnvalue_4 (`|SpawnActorFromClass` "/Game/InfiniteMatrix/Blueprints/BP_HealthPack.BP_HealthPack_C" (`KismetMathLibrary.MakeTransform` _returnvalue) "Undefined" "MultiplyWithRoot" null null))
    (`self.SetLifeSpan` _returnvalue_4 20.0)
    (`self.SetLifeSpan` _returnvalue_3 20.0)))

(fn `SpawnTunnelAtPoint`
  (`self.SpawnTunnel` (`SceneComponent.K2_GetComponentLocation` (`/Game/InfiniteMatrix/Blueprints/BP_Tunnel.SpawnPoint` (`self.NewestTunnel`)))))

(fn `UserConstructionScript`)