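; BP_Projectile is a projectile that destroys enemies on impact and awards the player score for each kill.
; The construction script sets the projectile movement's initial and maximum speed from a Speed variable.
; On component hit, it destroys itself against health packs and tunnels, while an enemy hit adds score to player pawn 0 and destroys both actors.
; Hits on any other actor leave the projectile alive.
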(event `self.Projectile.OnComponentHit`
  (params (HitComponent :type "PrimitiveComponent Object Reference") (OtherActor :type "Actor Object Reference") (OtherComp :type "PrimitiveComponent Object Reference") (NormalImpulse :type "Vector Structure") (Hit :type "HitResult Structure (by ref)"))
  (cast `/Game/InfiniteMatrix/Blueprints/BP_HealthPack` OtherActor
    (:`then`
      _)
    (:`CastFailed`
      (cast `/Game/InfiniteMatrix/Blueprints/BP_Tunnel` OtherActor
        (:`then`
          _)
        (:`CastFailed`
          (bind _asbp_enemy (cast `/Game/InfiniteMatrix/Blueprints/BP_Enemy` OtherActor))
          (bind _asbp_player (cast `/Game/InfiniteMatrix/Blueprints/BP_Player` (`GameplayStatics.GetPlayerPawn` 0)))
          (set `/Game/InfiniteMatrix/Blueprints/BP_Player.Score` (+ (`/Game/InfiniteMatrix/Blueprints/BP_Player.Score` _asbp_player) 150) _asbp_player)
          (`self.K2_DestroyActor` _asbp_enemy)))))
  (`self.K2_DestroyActor`))

(fn `UserConstructionScript`
  (bind _projectilemovement (`self.ProjectileMovement`))
  (bind _speed (`self.Speed`))
  (set `ProjectileMovementComponent.InitialSpeed` _speed _projectilemovement)
  (set `ProjectileMovementComponent.MaxSpeed` _speed _projectilemovement))