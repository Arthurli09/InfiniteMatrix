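; BP_Enemy is a contact-damage enemy actor that spins in place and hurts the player on collision.
; Tick yaws its static mesh at a steady rate scaled by delta time.
; On a mesh hit with BP_Player, it lowers and clamps the player's Health, destroys itself, and calls the player's DisplayRestart when health is nearly depleted.
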(event `self.ReceiveTick`
  (params (DeltaSeconds :type "Float (single-precision)"))
  (`SceneComponent.K2_AddLocalRotation` (`self.StaticMeshComponent`) (`KismetMathLibrary.MakeRotator` 0.0 0.0 (* DeltaSeconds 60.0)) false false))

(event `self.StaticMeshComponent.OnComponentHit`
  (params (HitComponent :type "PrimitiveComponent Object Reference") (OtherActor :type "Actor Object Reference") (OtherComp :type "PrimitiveComponent Object Reference") (NormalImpulse :type "Vector Structure") (Hit :type "HitResult Structure (by ref)"))
  (bind _asbp_player (cast `/Game/InfiniteMatrix/Blueprints/BP_Player` OtherActor))
  (bind _output_get (set `/Game/InfiniteMatrix/Blueprints/BP_Player.Health` (`KismetMathLibrary.FClamp` (- (`/Game/InfiniteMatrix/Blueprints/BP_Player.Health` _asbp_player) 0.1)) _asbp_player))
  (`self.K2_DestroyActor`)
  (if (< _output_get 0.1)
    (`/Game/InfiniteMatrix/Blueprints/BP_Player.DisplayRestart` _asbp_player)))

(fn `UserConstructionScript`)